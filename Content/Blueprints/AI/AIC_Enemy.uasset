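; AI controller for enemy characters that runs the enemy behavior tree on its blackboard.
; On possess it binds to the character's stun event and mirrors that state into the blackboard, alongside the attack target set through SetAttackTarget.
; Each tick it sets the focal point toward the target along world X only while the character can act, otherwise it holds the current forward direction.
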(event Custom|OnStunStateChanged
  (params (IsStunned :type Boolean))
  (AI|Components|Blackboard|SetValueasBool (Variables|Default|GetBlackboard) (Variables|Default|GetIsStunnedKey) IsStunned))

(event EventBeginPlay
  (Class|AIController|UseBlackboard "/Game/Blueprints/AI/BB_Enemy.BB_Enemy")
  (AI|RunBehaviorTree "/Game/Blueprints/AI/BT_Enemy.BT_Enemy"))

(event EventPossess
  (params (PossessedPawn :type Pawn%20Object%20Reference))
  (bind _asbp_character (Utilities|Casting|CastToBP_Character PossessedPawn))
  (bind _output_get (Variables|Default|SetActionCharacter _asbp_character))
  (EventDispatchers|BindEventtoStunStateChanged _output_get (delegate Custom|OnStunStateChanged)))

(event EventTick
  (params (DeltaSeconds :type Float%20%28single-precision%29))
  (CallFunction|SetFocusDirection))

(fn ConstructionScript)

(fn SetAttackTarget
  (params (AttackTarget :type BP%20Captain%20Object%20Reference))
  (AI|Components|Blackboard|SetValueasObject (Variables|Default|GetBlackboard) (Variables|Default|GetAttackTargetKey) AttackTarget)
  (Variables|Default|SetAttackTarget AttackTarget))

(fn SetFocusDirection
  (bind _actioncharacter (Variables|Default|GetActionCharacter))
  (Utilities|IsValid (Variables|Default|GetAttackTarget)
    (:Is%20Valid
      (if (Default|CanAct (Variables|Default|GetActionCharacter))
        (AI|SetFocalPoint (+ (Transformation|GetActorLocation (Variables|Default|GetActionCharacter)) (Math|Vector|MakeVector (.x (Math|Vector|GetForwardVector (Math|Rotator|FindLookatRotation (Transformation|GetActorLocation (Variables|Default|GetActionCharacter)) (Transformation|GetActorLocation (Variables|Default|GetAttackTarget))))) 0.0 0.0)))
        (else
          (AI|SetFocalPoint (+ (Transformation|GetActorLocation _actioncharacter) (Transformation|GetActorForwardVector _actioncharacter)) :!label _label))))
    (:Is%20Not%20Valid
      (goto _label))))